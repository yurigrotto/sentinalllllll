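; BP_Door_Locked is a locked door actor with a keypad UI, though its door-movement Timeline is unwired.
; Player overlap with its Box enables input, letting E flip-flop between creating a WBP_Keypad with cursor and removing it.
; Leaving the Box calls DisableInput on the controller and shares that removal path, restoring game-only input.
; The Keypad variable assignment never runs, so removal lacks the created widget, and nothing hides the cursor.
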(event OnComponentBeginOverlap(Box)
  (params (OverlappedComponent :type Primitive%20Component%20Object%20Reference) (OtherActor :type Actor%20Object%20Reference) (OtherComp :type Primitive%20Component%20Object%20Reference) (OtherBodyIndex :type Integer) (bFromSweep :type Boolean) (SweepResult :type Hit%20Result%20Structure%20%28by%20ref%29))
  (Utilities|Casting|CastToPlayerCharacter OtherActor)
  (Input|EnableInput (Game|GetPlayerController 0)))

(event OnComponentEndOverlap(Box)
  (params (OverlappedComponent :type Primitive%20Component%20Object%20Reference) (OtherActor :type Actor%20Object%20Reference) (OtherComp :type Primitive%20Component%20Object%20Reference) (OtherBodyIndex :type Integer))
  (Utilities|Casting|CastToPlayerCharacter OtherActor)
  (Input|DisableInput (Game|GetPlayerController 0) 0)
  (Widget|RemovefromParent (Variables|Default|GetKeypad))
  (Input|SetInputModeGameOnly (Game|GetPlayerController 0) false))

(event Input|KeyboardEvents|E
  (params (Key :type Key%20Structure :default "None"))
  (bind _returnvalue (Game|GetPlayerController 0))
  (:Pressed
    (Utilities|FlowControl|FlipFlop
      (:A
        (bind _returnvalue_2 (UserInterface|CreateWidget "/Game/StudentWork/widgets/WBP_Keypad.WBP_Keypad_C"))
        (UserInterface|Viewport|AddtoViewport _returnvalue_2 0)
        (Input|SetInputModeGameandUI _returnvalue _returnvalue_2 "DoNotLock" true false)
        (Variables|/Script/Engine.PlayerController|SetbShowMouseCursor _returnvalue true))
      (:B
        (Widget|RemovefromParent (Variables|Default|GetKeypad))
        (Input|SetInputModeGameOnly _returnvalue false)))))

(fn ConstructionScript)