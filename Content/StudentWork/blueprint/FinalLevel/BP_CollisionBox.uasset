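; BP_CollisionBox is a trigger volume for the final level that switches the camera view and shows a countdown.
; On overlap it blends player 0's view to Camera, adds a WBP_FinalLevel widget and starts a looping timer.
; Countdown decrements Count and writes it to the widget text, but reaching zero triggers nothing.
; Ending overlap blends the view to the exiting actor, leaving the timer and widget in place.
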(event OnComponentBeginOverlap(Box)
  (params (OverlappedComponent :type Primitive%20Component%20Object%20Reference) (OtherActor :type Actor%20Object%20Reference) (OtherComp :type Primitive%20Component%20Object%20Reference) (OtherBodyIndex :type Integer) (bFromSweep :type Boolean) (SweepResult :type Hit%20Result%20Structure%20%28by%20ref%29))
  (Game|Player|SetViewTargetwithBlend (Game|GetPlayerController 0) (Variables|Default|GetCamera) 2.0 "VTBlend_Linear" 0.0 false)
  (bind _returnvalue (UserInterface|CreateWidget "/Game/StudentWork/widgets/WBP_FinalLevel.WBP_FinalLevel_C"))
  (bind _output_get (Variables|Default|SetTimerWidget _returnvalue))
  (UserInterface|Viewport|AddtoViewport _output_get 0)
  (Utilities|Time|SetTimerbyEvent (delegate Custom|Countdown) 0.0 true))

(event OnComponentEndOverlap(Box)
  (params (OverlappedComponent :type Primitive%20Component%20Object%20Reference) (OtherActor :type Actor%20Object%20Reference) (OtherComp :type Primitive%20Component%20Object%20Reference) (OtherBodyIndex :type Integer))
  (Game|Player|SetViewTargetwithBlend (Game|GetPlayerController 0) OtherActor 2.0 "VTBlend_Linear" 0.0 false))

(event Custom|Countdown
  (Math|Integer|DecrementInt (Variables|Default|GetCount)
    (:%20%20
      (Rendering|Components|TextRender|SetText (Variables|/Game/StudentWork/widgets/WBP_FinalLevel.WBP_FinalLevel_C|GetTXT_Timer (Variables|Default|GetTimerWidget)) (Utilities|Text|ToText(Integer) (Variables|Default|GetCount)))
      (if (<= (Variables|Default|GetCount) 0)
        _))))

(fn ConstructionScript)