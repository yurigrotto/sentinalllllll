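; BP_Door is a door that slides open when something enters its trigger box and closes when it leaves.
; BeginPlay stores the mesh's start location; box overlap plays a Timeline and end overlap reverses it.
; Each Timeline update lerps the static mesh in world space between the start and the start plus a TargetPos offset, without filtering the overlapping actor.
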(event OnComponentBeginOverlap(Box)
  (params (OverlappedComponent :type Primitive%20Component%20Object%20Reference) (OtherActor :type Actor%20Object%20Reference) (OtherComp :type Primitive%20Component%20Object%20Reference) (OtherBodyIndex :type Integer) (bFromSweep :type Boolean) (SweepResult :type Hit%20Result%20Structure%20%28by%20ref%29))
  (bind _startpos (Variables|Default|GetStartPos))
  (bind _alpha (Timeline|Timeline Play)
    (:Update
      (Transformation|SetWorldLocation (Variables|Default|GetStaticMesh) (Math|Vector|Lerp(Vector) _startpos (+ _startpos (Variables|Default|GetTargetPos)) _alpha) false false))))

(event OnComponentEndOverlap(Box)
  (params (OverlappedComponent :type Primitive%20Component%20Object%20Reference) (OtherActor :type Actor%20Object%20Reference) (OtherComp :type Primitive%20Component%20Object%20Reference) (OtherBodyIndex :type Integer))
  (bind _startpos (Variables|Default|GetStartPos))
  (bind _alpha (Timeline|Timeline Reverse)
    (:Update
      (Transformation|SetWorldLocation (Variables|Default|GetStaticMesh) (Math|Vector|Lerp(Vector) _startpos (+ _startpos (Variables|Default|GetTargetPos)) _alpha) false false))))

(event EventBeginPlay
  (Variables|Default|SetStartPos (Transformation|GetWorldLocation (Variables|Default|GetStaticMesh))))

(fn ConstructionScript)