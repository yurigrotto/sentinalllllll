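; Player controller that runs a level session: input setup, fade-in, respawning, run stats and level end.
; On BeginPlay it caches the first PlayerStart as spawn point, defaults the next level to the current one and starts a one-second timer.
; IA_Respawn replaces a dead or invalid pawn at that point, re-granting a held shield via a spawned pickup.
; EndScreen formats the time and shows the end widget; ProgressLevel opens the target level.
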(event Custom|LevelTimerEvent
  ;[1 1 1] Level Timer Countup
  (Variables|Timer|SetLevelTimer (+ (Variables|Timer|GetLevelTimer) 1)))

(event Custom|DeathCounterEvent
  ;[1 1 1] Death Counter
  (Variables|Default|SetDeathCounter (+ (Variables|Default|GetDeathCounter) 1)))

(event Custom|EndScreen
  ;[1 1 1] Show End Screen UI
  (Variables|/Game/Blueprints/PlayerCharacter.PlayerCharacter_C|SetUIMode (Variables|Default|GetMyPlayer) true)
  (Utilities|Time|ClearTimerbyFunctionName 0 "LevelTimerEvent")
  (CallFunction|TimerConversion (Variables|Timer|GetLevelTimer))
  (bind _returnvalue (UserInterface|CreateWidget "/Game/UI/WBP_EndScreen.WBP_EndScreen_C"))
  (bind _output_get (Variables|Default|SetEndScreenUI _returnvalue))
  (UserInterface|Viewport|AddtoViewport _output_get 0)
  (Input|SetInputModeUIOnly (Game|GetPlayerController 0) _returnvalue "DoNotLock" false))

(event Custom|ProgressLevel
  ;[1 1 1] Level Progression
  (Widget|RemovefromParent (Variables|Default|GetEndScreenUI))
  (Game|OpenLevel(byName) (Variables|Default|GetTargetLevelProgression)))

(event Custom|Give%20Shield
  (Utilities|FlowControl|Delay 0.2)
  (bind _returnvalue (Game|SpawnActorfromClass "/Game/Blueprints/MiscBlueprints/BP_ShieldPickUp.BP_ShieldPickUp_C" (Math|Transform|MakeTransform "0, 0, 0" "0, 0, 0" "1.000000,1.000000,1.000000") "Undefined" "OverrideRootScale" 0 0))
  (Default|PickedUp _returnvalue (Variables|Default|GetMyPlayer)))

(event Input|EnhancedActionEvents|EnhancedInputActionIA_Respawn
  (params (ActionValue :type Boolean) (ElapsedSeconds :type Float%20%28double-precision%29) (TriggeredSeconds :type Float%20%28double-precision%29) (InputAction :type Input%20Action%20Object%20Reference :default "/Game/Blueprints/MiscBlueprints/Inputs/IA_Respawn.IA_Respawn"))
  ;[1 1 1] Respawn Player
  (:Started
    (Utilities|IsValid (Variables|Default|GetMyPlayer)
      (:Is%20Valid
        (if (Variables|/Game/Blueprints/PlayerCharacter.PlayerCharacter_C|GetDead (Variables|Default|GetMyPlayer))
          (Widget|RemovefromParent (Variables|/Game/Blueprints/PlayerCharacter.PlayerCharacter_C|GetMyUI (Variables|Default|GetMyPlayer)))
          (Variables|Default|SetPlayerHadShield (Variables|/Game/Blueprints/PlayerCharacter.PlayerCharacter_C|GetCanShield (Variables|Default|GetMyPlayer)))
          (Actor|DestroyActor (Variables|Default|GetMyPlayer))
          (bind _returnvalue (Game|SpawnActorfromClass "/Game/Blueprints/PlayerCharacter.PlayerCharacter_C" (Math|Transform|MakeTransform (Variables|Default|GetSpawnPoint) "0, 0, 0" "1.000000,1.000000,1.000000") "AdjustIfPossibleButAlwaysSpawn" "MultiplyWithRoot" 0 0 :!label _label))
          (bind _output_get (Variables|Default|SetMyPlayer _returnvalue))
          (Pawn|Possess _output_get)
          (Default|InitPlayer _output_get)
          (CameraFades|StartCameraFade (Game|GetPlayerCameraManager 0) 2.0 0.0 0.9 "(R=0.000000,G=0.000000,B=0.000000,A=1.000000)" false false)
          (if (Variables|Default|GetPlayerHadShield)
            (CallFunction|GiveShield))))
      (:Is%20Not%20Valid
        (Viewport|RemoveAllWidgets)
        (goto _label)))))

(event EventBeginPlay
  (bind _returnvalue (Game|GetPlayerCameraManager 0))
  ;[1 1 1] Begin Play - Character Initialise
  (Input|AddMappingContext (PlayerController|LocalPlayerSubsystems|GetEnhancedInputLocalPlayerSubsystem) "/Game/Blueprints/MiscBlueprints/Inputs/IMC_Default.IMC_Default" 0 "(bIgnoreAllPressedKeysUntilRelease=True,bForceImmediately=False,bNotifyUserSettings=False)")
  (Utilities|FlowControl|Sequence
    (:then_0
      ;;[1 1 1] Initialise the Spawn Point
      (bind _outactors (Actor|GetAllActorsOfClass "/Script/Engine.PlayerStart"))
      (Variables|Default|SetSpawnPoint (Transformation|GetActorLocation (Utilities|Array|Get(acopy) _outactors))))
    (:then_1
      ;;[1 1 1] Set Default Level Progression
      (bind _returnvalue_2 (Game|GetCurrentLevelName true))
      (Variables|Default|SetTargetLevelProgression (Utilities|String|StringToName _returnvalue_2)))
    (:then_2
      ;;[1 1 1] Cast to the Player Character
      (bind _asplayer_character (Utilities|Casting|CastToPlayerCharacter (Pawn|GetControlledPawn)))
      (Variables|Default|SetMyPlayer _asplayer_character))
    (:then_3
      ;;[1 1 1] Init Camera Fade
      (CameraFades|StartCameraFade :self _returnvalue :FromAlpha 1.0 :ToAlpha 1.0 :Duration 0.1 :bHoldWhenFinished true)
      (Utilities|FlowControl|Delay 0.5)
      (CameraFades|StartCameraFade :self _returnvalue :FromAlpha 1.0 :Duration 2.0))
    (:then_4
      ;;[1 1 1] Level Counter Timer Init
      (Utilities|Time|SetTimerbyFunctionName 0 "LevelTimerEvent" 1.0 true))
    (:then_5
      (Input|SetInputModeGameandUI (Game|GetPlayerController 0) 0 "DoNotLock" false false))))

(fn ConstructionScript)

(fn TimerConversion
  (params (CurrentTimeCounter :type Integer))
  (bind _returnvalue (Math|Conversions|ToFloat(Integer) CurrentTimeCounter))
  (bind _returnvalue_2 (/ _returnvalue 6e+01))
  (bind _returnvalue_3 (Math|Float|%(Float) _returnvalue 6e+01))
  (bind _returnvalue_4 (Math|Float|Floor _returnvalue_3))
  (bind _returnvalue_5 (Math|Float|Floor _returnvalue_2))
  (bind _output_get (Variables|Timer|SetEndScreenTime (Utilities|Text|ToText(String) (Utilities|String|Append (Utilities|String|Append (Utilities|String|SelectString (Utilities|String|Append "0" (Utilities|String|ToString(Integer) _returnvalue_5)) (Utilities|String|ToString(Integer) _returnvalue_5) (< _returnvalue_5 9)) ":") (Utilities|String|ToString(Text) (Utilities|Text|ToText(Integer) (Math|Conversions|ToInteger(Byte) (Utilities|String|SelectString (Utilities|String|ToString(Integer) _returnvalue_4) (Utilities|String|ToString(Integer) _returnvalue_4) (> _returnvalue_4 9))) false true 2))))))
  (return _output_get))