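; BP_Shield is a shield actor that grows a sphere mesh into view on spawn and shrinks it away when deactivated.
; Activate plays or reverses a sped-up timeline that lerps the sphere's scale between zero and slightly oversized, destroying the actor when the reverse finishes.
; The construction script gives the sphere a dynamic shield material instance with a bright cyan HDR colour.
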(event Custom|Activate
  (params (On? :type Boolean))
  (Components|Timeline|SetPlayRate (Variables|Default|GetShield%20Grow%20TL) 6.0)
  (if On?
    (bind (_direction _alpha) (Timeline|Shield%20Grow%20TL Play)
      (:Update
        (Transformation|SetWorldScale3D (Variables|Default|GetSphere) (Math|Vector|Lerp(Vector) "0, 0, 0" "1.200000,1.200000,1.200000" _alpha)))
      (:Finished
        (switch Utilities|FlowControl|Switch|SwitchonETimelineDirection _direction
          (:Backward
            (Actor|DestroyActor)))))
    (else
      (Timeline|Shield%20Grow%20TL Reverse))))

(event EventBeginPlay
  (CallFunction|Activate true))

(fn ConstructionScript
  (bind _returnvalue (Rendering|Material|CreateDynamicMaterialInstance (Variables|Default|GetSphere) 0 "/Game/Materials/MI_ShieldMaster.MI_ShieldMaster" "None" :!class /Script/Engine.PrimitiveComponent))
  (bind _output_get (Variables|Default|SetMyMaterial _returnvalue))
  (Rendering|Material|SetVectorParameterValue _output_get "Colour" "(R=3.100000,G=29.000000,B=27.000000,A=1.000000)" :!class /Script/Engine.MaterialInstanceDynamic))